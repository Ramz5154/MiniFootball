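; Field spotlight for the mini-football game that flashes when a goal is scored.
; On BeginPlay it registers itself with GM_MiniFootballGameMode.
; OnGoalScored switches on Team and alternates the light between white and a color through chained delays, ending on white.
; The Blue case flashes red and the Red case flashes blue.
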(event Custom|OnGoalScored
  (params (team :type E_teams%20Enum :default "NewEnumerator0"))
  (bind _spotlightcomponent (Variables|Default|GetSpotLightComponent))
  (bind _spotlightcomponent_2 (Variables|Default|GetSpotLightComponent))
  (switch Utilities|FlowControl|Switch|SwitchonE_teams team
    (:NewEnumerator0
      (Rendering|Components|Light|SetLightColor _spotlightcomponent "(R=1.000000,G=1.000000,B=1.000000,A=1.000000)" true)
      (Utilities|FlowControl|Delay 0.4)
      (Rendering|Components|Light|SetLightColor _spotlightcomponent "(R=1.000000,G=0.000000,B=0.004421,A=1.000000)" true)
      (Utilities|FlowControl|Delay 0.4)
      (Rendering|Components|Light|SetLightColor _spotlightcomponent "(R=1.000000,G=1.000000,B=1.000000,A=1.000000)" true)
      (Utilities|FlowControl|Delay 0.4)
      (Rendering|Components|Light|SetLightColor _spotlightcomponent "(R=1.000000,G=0.000000,B=0.000000,A=1.000000)" true)
      (Utilities|FlowControl|Delay 0.4)
      (Rendering|Components|Light|SetLightColor _spotlightcomponent "(R=1.000000,G=1.000000,B=1.000000,A=1.000000)" true)
      (Utilities|FlowControl|Delay 0.4)
      (Rendering|Components|Light|SetLightColor _spotlightcomponent "(R=1.000000,G=0.000000,B=0.000000,A=1.000000)" true)
      (Utilities|FlowControl|Delay 0.4)
      (Rendering|Components|Light|SetLightColor _spotlightcomponent "(R=1.000000,G=1.000000,B=1.000000,A=1.000000)" true))
    (:NewEnumerator1
      (Rendering|Components|Light|SetLightColor _spotlightcomponent_2 "(R=1.000000,G=1.000000,B=1.000000,A=1.000000)" true)
      (Utilities|FlowControl|Delay 0.4)
      (Rendering|Components|Light|SetLightColor _spotlightcomponent_2 "(R=0.000000,G=0.019749,B=1.000000,A=1.000000)" true)
      (Utilities|FlowControl|Delay 0.4)
      (Rendering|Components|Light|SetLightColor _spotlightcomponent_2 "(R=1.000000,G=1.000000,B=1.000000,A=1.000000)" true)
      (Utilities|FlowControl|Delay 0.4)
      (Rendering|Components|Light|SetLightColor _spotlightcomponent_2 "(R=0.000000,G=0.073006,B=1.000000,A=1.000000)" true)
      (Utilities|FlowControl|Delay 0.4)
      (Rendering|Components|Light|SetLightColor _spotlightcomponent_2 "(R=1.000000,G=1.000000,B=1.000000,A=1.000000)" true)
      (Utilities|FlowControl|Delay 0.2)
      (Rendering|Components|Light|SetLightColor _spotlightcomponent_2 "(R=0.000000,G=0.073006,B=1.000000,A=1.000000)" true)
      (Utilities|FlowControl|Delay 0.4)
      (Rendering|Components|Light|SetLightColor _spotlightcomponent_2 "(R=1.000000,G=1.000000,B=1.000000,A=1.000000)" true))))

(event EventBeginPlay
  (bind _asgm_mini_football_game_mode (Utilities|Casting|CastToGM_MiniFootballGameMode (Game|GetGameMode)))
  (Default|RegisterLights _asgm_mini_football_game_mode self))

(fn ConstructionScript)