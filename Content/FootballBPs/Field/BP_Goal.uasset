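; BP_Goal is a football goal actor that detects when the ball enters its trigger and reports a score for its team.
; On server authority, an overlap with BP_FootBall prints debug text and passes the goal's Team to GM_MiniFootballGameMode's GoalScoredEvents.
; It then fires a multicast event that plays a placeholder sine-tone sound at the net mesh's relative location on all machines.
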(event OnComponentBeginOverlap(GoalCollisionTrigger)
  (params (OverlappedComponent :type Primitive%20Component%20Object%20Reference) (OtherActor :type Actor%20Object%20Reference) (OtherComp :type Primitive%20Component%20Object%20Reference) (OtherBodyIndex :type Integer) (bFromSweep :type Boolean) (SweepResult :type Hit%20Result%20Structure%20%28by%20ref%29))
  (Networking|SwitchHasAuthority
    (:Authority
      (Utilities|Casting|CastToBP_FootBall OtherActor)
      (Development|PrintString "goal triggered")
      (Development|PrintString (Utilities|String|EnumtoString (Variables|Default|GetTeam)))
      (bind _asgm_mini_football_game_mode (Utilities|Casting|CastToGM_MiniFootballGameMode (Game|GetGameMode)))
      (Default|GoalScoredEvents _asgm_mini_football_game_mode (Variables|Default|GetTeam))
      (CallFunction|MulticastonGoalScored))))

(event Custom|Multicast_OnGoalScored
  (Audio|PlaySoundatLocation "/Engine/EngineSounds/1kSineTonePing.1kSineTonePing" (Variables|/Script/Engine.SceneComponent|GetRelativeLocation (Variables|Default|GetSM_net)) "0, 0, 0" 1.0 1.0 0.0 0 0 0 0))

(fn ConstructionScript)