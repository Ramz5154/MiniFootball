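; Physics football for a networked mini football game, with impulse-based kick, lob and dribble shots.
; The server records the ball's location and velocity every tick.
; On location RepNotify, the actor snaps to the server position while the mesh takes the offset, which remote ticks interpolate to zero for smooth correction.
; A server-side reset destroys the ball and asks GM_MiniFootballGameMode to respawn it.
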(event Custom|applyKick
  (params (kickDirection :type Vector))
  ;[1 1 1] Types of shots/ ball mechanics
  (Physics|AddImpulse (Variables|Default|GetSC_football) (* kickDirection 1400) "None" true))

(event Custom|ServerResetBall
  (Networking|SwitchHasAuthority
    (:Authority
      (bind _outactors (Actor|GetAllActorsOfClass "BP_FootBall_C"))
      (for _array_element _outactors
        (Actor|DestroyActor))
      (bind _asgm_mini_football_game_mode (Utilities|Casting|CastToGM_MiniFootballGameMode (Game|GetGameMode)))
      (Default|RespawnBall _asgm_mini_football_game_mode))))

(event Custom|ApplyLobKick
  (params (kickDirection :type Vector))
  ;[1 1 1] Types of shots/ ball mechanics
  (Physics|AddImpulse (Variables|Default|GetSC_football) (+ (* kickDirection "500.000000,0.000000,2000.000000") "2.000000,0.000000,1000.000000") "None" true)
  (Development|PrintString "lobkicked"))

(event Custom|ApplyDribble
  (params (kickDirection :type Vector))
  ;[1 1 1] Types of shots/ ball mechanics
  (Physics|AddImpulse (Variables|Default|GetSC_football) (+ (* kickDirection "0.000000,0.000000,2000.000000") "0.000000,0.000000,500.000000") "None" true)
  (Development|PrintString "dribble"))

(event EventTick
  (params (DeltaSeconds :type Float%20%28single-precision%29))
  (bind _sm_football (Variables|Default|GetSM_Football))
  (Networking|SwitchHasAuthority
    (:Authority
      (Variables|Default|SetServerLocation (Transformation|GetActorLocation))
      (bind _returnvalue (Physics|GetPhysicsLinearVelocity (Variables|Default|GetSC_football) "None"))
      (Variables|Default|SetServerVelocity _returnvalue))
    (:Remote
      (Transformation|SetRelativeLocation _sm_football (Math|Interpolation|VInterpTo (Variables|/Script/Engine.SceneComponent|GetRelativeLocation _sm_football) "0, 0, 0" DeltaSeconds 17.0) false false))))

(fn ConstructionScript)

(fn OnRepServerLocation
  (bind _serverlocation (Variables|Default|GetServerLocation))
  (Variables|Default|SettargetLocation (Variables|Default|GetServerLocation))
  (LocalVariables|SetTargetVelocity (Variables|Default|GetServerVelocity))
  (Variables|Default|Setvisual%20offset (- (Transformation|GetActorLocation) _serverlocation))
  (Transformation|SetActorLocation _serverlocation false false)
  (Transformation|SetRelativeLocation (Variables|Default|GetSM_Football) (Variables|Default|Getvisual%20offset) false false))