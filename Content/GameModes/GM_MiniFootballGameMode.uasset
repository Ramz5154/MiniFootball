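; Game mode for a mini football match that spawns players, handles goals and resets the pitch.
; Each joining player possesses a new BP_Striker at the PlayerStart matching the join count, with teams alternating by parity.
; Goals update the game state's score and widget and destroy balls.
; After timed delays, it destroys all strikers, resets the count, spawns a ball at the cached Bp_ballspawn transform and respawns every stored controller.
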(event Custom|goalScoredEvents
  (params (teams :type E_teams%20Enum :default "NewEnumerator0"))
  (CallFunction|HandlegoalScored teams)
  (Utilities|FlowControl|Delay 4.0)
  (CallFunction|Dest)
  (Utilities|FlowControl|Delay 3.0)
  (CallFunction|RespawnBall)
  (for _array_element (Variables|Default|GetPlayerControllers)
    (CallFunction|SpawnPlayers "NewEnumerator0" _array_element)))

(event Custom|SpawnPlayers
  (params (team :type E_teams%20Enum :default "NewEnumerator0") (player%20controller :type Player%20Controller%20Object%20Reference))
  (bind _returnvalue (Game|SpawnActorfromClass "/Game/PlayersBPs/BP_Striker.BP_Striker_C" (Transformation|GetActorTransform (Utilities|Array|Get(acopy) (Variables|Default|GetPlayerStartLocations) (Variables|Default|GetplayersJoined))) "Undefined" "MultiplyWithRoot" 0 0))
  (if (== (Math|Integer|%(Integer) (Variables|Default|GetplayersJoined) 2) 1)
    (Variables|Default|Setteam "NewEnumerator0")
    (else
      (Variables|Default|Setteam "NewEnumerator1")))
  (Variables|/Game/PlayersBPs/BP_Striker.BP_Striker_C|SetTeam _returnvalue (Variables|Default|Getteam))
  (Pawn|Possess player%20controller _returnvalue)
  (bind _result (Math|Integer|IncrementInt (Variables|Default|GetplayersJoined))
    (:%20%20
      (Variables|Default|SetplayersJoined _result))))

(event EventBeginPlay
  (bind _returnvalue (Actor|GetActorOfClass "/Game/FootballBPs/Field/bp_ballspawn.bp_ballspawn_C"))
  (Variables|Default|SetballSpawn (Transformation|GetActorTransform _returnvalue)))

(event EventPostLogin
  (params (NewPlayer :type Player%20Controller%20Object%20Reference))
  (Utilities|Array|AddUnique (Variables|Default|GetPlayerControllers) NewPlayer)
  (bind _outactors (Actor|GetAllActorsOfClass "/Script/Engine.PlayerStart"))
  (Variables|Default|SetPlayerStartLocations _outactors)
  (CallFunction|SpawnPlayers "NewEnumerator1" NewPlayer))

(fn ConstructionScript)

(fn HandlegoalScored
  (params (teams :type E_teams%20Enum :default "NewEnumerator0"))
  (bind _asgs_mini_football_game_state (Utilities|Casting|CastToGS_miniFootballGameState (Game|GetGameState))
    (:then
      (Variables|/Game/GameModes/GS_miniFootballGameState.GS_miniFootballGameState_C|SetLastScoringTeam _asgs_mini_football_game_state teams)
      (Default|AddScore _asgs_mini_football_game_state teams)
      (bind _result (Math|Integer|IncrementInt (Variables|/Game/GameModes/GS_miniFootballGameState.GS_miniFootballGameState_C|GettotalGoals _asgs_mini_football_game_state))
        (:%20%20
          ;[1 1 1] runs the spotlights
          (Variables|/Game/GameModes/GS_miniFootballGameState.GS_miniFootballGameState_C|SettotalGoals _asgs_mini_football_game_state _result)
          (Default|ShowGoalScoreWidget _asgs_mini_football_game_state)
          (Development|PrintString "goal scored gamemode")
          (bind _outactors (Actor|GetAllActorsOfClass "/Game/FootballBPs/BP_FootBall.BP_FootBall_C"))
          (for _array_element _outactors
            (Actor|DestroyActor _array_element)))))
    (:CastFailed
      (Development|PrintString "cast to gamestate failed"))))

(fn RespawnBall
  (Game|SpawnActorfromClass "/Game/FootballBPs/BP_FootBall.BP_FootBall_C" (Variables|Default|GetballSpawn) "Undefined" "MultiplyWithRoot" 0 0))

(fn Dest
  (bind _outactors (Actor|GetAllActorsOfClass "/Game/PlayersBPs/BP_Striker.BP_Striker_C"))
  (for _array_element _outactors
    (Actor|DestroyActor _array_element)
    (Variables|Default|SetplayersJoined 0)))